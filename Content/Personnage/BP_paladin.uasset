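; Player paladin character handling movement, sprint, crouch, health with death, and a "surprise" dance with music that attacks cancel.
; Camera-forward sphere traces open doors and pick up items, while box traces damage enemies as light or heavy attack montages start, without waiting for impact.
; Pickups go into a struct-array inventory that stacks stackable items by name and rebuilds the toggleable bag widget from that array.
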(event Input|ActionEvents|InputActionJump
  (params (Key :type Key%20Structure))
  ;[1 1 1] saut
  (:Pressed
    (Character|Jump))
  (:Released
    (Character|StopJumping)))

(event Input|ActionEvents|InputActionsprint
  (params (Key :type Key%20Structure))
  (bind _charactermovement (Variables|Character|GetCharacterMovement))
  ;[1 1 1] sprint
  (:Pressed
    (Variables|/Script/Engine.CharacterMovementComponent|SetMaxWalkSpeed _charactermovement 6e+02))
  (:Released
    (Variables|/Script/Engine.CharacterMovementComponent|SetMaxWalkSpeed _charactermovement 2.4e+02)))

(event Input|ActionEvents|InputActioncrouch
  (params (Key :type Key%20Structure))
  ;[1 1 1] crouch
  (:Pressed
    (Character|Crouch))
  (:Released
    (Character|UnCrouch)))

(event Input|ActionEvents|InputActionramasser
  (params (Key :type Key%20Structure))
  ;[1 1 1] ramasser item
  (:Pressed
    (CallFunction|RamasserItem)))

(event Input|ActionEvents|InputActionOuverture_inventaire
  (params (Key :type Key%20Structure))
  ;[1 1 1] inventaire
  (:Pressed
    (Utilities|IsValid (Variables|Default|GetUI_BagRef)
      (:Is%20Valid
        (Utilities|FlowControl|FlipFlop
          (:A
            (Widget|RemovefromParent (Variables|Default|GetUI_BagRef))
            (Variables|/Script/Engine.PlayerController|SetbShowMouseCursor (Game|GetPlayerController 0) false))
          (:B
            (UserInterface|Viewport|AddtoViewport (Variables|Default|GetUI_BagRef) 0)
            (CallFunction|ChargerInventaire)
            (Variables|/Script/Engine.PlayerController|SetbShowMouseCursor (Game|GetPlayerController 0) true :!label _label))))
      (:Is%20Not%20Valid
        (bind _returnvalue (UserInterface|CreateWidget "/Game/HUD/UI_bag.UI_bag_C"))
        (bind _output_get (Variables|Default|SetUI_BagRef _returnvalue))
        (UserInterface|Viewport|AddtoViewport _output_get 0)
        (CallFunction|ChargerInventaire)
        (goto _label)))))

(event Input|ActionEvents|InputActionattack
  (params (Key :type Key%20Structure))
  ;[1 1 1] attack
  (:Pressed
    (bind _output_get (Variables|Default|Sethit true))
    (Animation|Montage|PlayMontage (Variables|Character|GetMesh) "/Game/Personnage/animation/Stable_Sword_Outward_Slash_Montage.Stable_Sword_Outward_Slash_Montage"
      (:then
        (if (stale Input|ActionEvents|InputActionsuprise _output_get)
          ;[1 1 1] stop animation
          (Audio|Components|Audio|Stop (stale Input|ActionEvents|InputActionsuprise _returnvalue))
          (Animation|StopAnimMontage 0)
          (Components|Activation|Activate (Variables|Character|GetCharacterMovement) true)
          (Variables|Default|Setsprise? false)
          (else
            (bind _asbp_ennemy (|CollapseGraph_0))
            (CallFunction|Infligdegat _asbp_ennemy 25.0)
            (if (> (Variables|Default|Getvie) 0.0)
              _))))
      (:OnBlendOut
        (if _output_get
          _)))))

(event Input|ActionEvents|InputActionsuprise
  (params (Key :type Key%20Structure))
  ;[1 1 1] dance
  (:Pressed
    (bind _output_get (Variables|Default|Setsprise? true))
    (Utilities|FlowControl|FlipFlop
      (:A
        (bind _returnvalue (Audio|SpawnSound2D "/Game/sons/persona-4-specialist_bmQt4Dcu.persona-4-specialist_bmQt4Dcu" 1.0 1.0 0.0 0))
        (Animation|Montage|PlayMontage (Variables|Character|GetMesh) "/Game/Personnage/animation/Northern_Soul_Spin_Combo_Montage.Northern_Soul_Spin_Combo_Montage"
          (:then
            (Components|Activation|Deactivate (Variables|Character|GetCharacterMovement)))))
      (:B
        (Audio|Components|Audio|Stop _returnvalue)
        (Animation|StopAnimMontage 0)
        (Components|Activation|Activate (Variables|Character|GetCharacterMovement) true)))))

(event Input|ActionEvents|InputActionattack_forte
  (params (Key :type Key%20Structure))
  ;[1 1 1] attack
  (:Pressed
    (Animation|Montage|PlayMontage (Variables|Character|GetMesh) "/Game/Personnage/animation/Great_Sword_Casting_Montage.Great_Sword_Casting_Montage"
      (:then
        (if (stale Input|ActionEvents|InputActionsuprise _output_get)
          ;[1 1 1] stop animation
          (Audio|Components|Audio|Stop (stale Input|ActionEvents|InputActionsuprise _returnvalue))
          (Animation|StopAnimMontage 0)
          (Components|Activation|Activate (Variables|Character|GetCharacterMovement) true)
          (Variables|Default|Setsprise? false)
          (else
            (bind _asbp_ennemy (|CollapseGraph_0_2))
            (CallFunction|Infligdegat _asbp_ennemy 5e+01)
            (if (> (Variables|Default|Getvie) 0.0)
              _)))))))

(event Input|ActionEvents|InputActioninteraction
  (params (Key :type Key%20Structure))
  (bind _camera (Variables|Default|GetCamera))
  (bind _camera_2 (Variables|Default|GetCamera))
  ;[1 1 1] ouverture porte
  (:Pressed
    (bind _outhit (Collision|SphereTraceByChannel (+ (Transformation|GetWorldLocation _camera_2) (* (Math|Vector|GetForwardVector _camera_2) 330)) (+ (Transformation|GetWorldLocation _camera) (* (Math|Vector|GetForwardVector _camera) 550)) 25.0 "TraceTypeQuery1" false 0 "None"))
    (bind _asbp_door (Utilities|Casting|CastToBP_door (.HitActor (Collision|BreakHitResult _outhit))))
    (Default|Dooriteraction _asbp_door)))

(event Input|AxisEvents|InputAxisMoveForward
  (params (AxisValue :type Float%20%28single-precision%29))
  ;[1 1 1] deplacement
  (Pawn|Input|AddMovementInput (Math|Vector|GetForwardVector (Math|Rotator|MakeRotator 0.0 0.0 (.Yaw (Math|Rotator|BreakRotator (Pawn|GetControlRotation :!class /Script/Engine.Pawn))))) AxisValue false))

(event Input|AxisEvents|InputAxisMoveRight
  (params (AxisValue :type Float%20%28single-precision%29))
  ;[1 1 1] deplacement
  (Pawn|Input|AddMovementInput (Math|Vector|GetRightVector (Math|Rotator|MakeRotator 0.0 0.0 (.Yaw (Math|Rotator|BreakRotator (Pawn|GetControlRotation :!class /Script/Engine.Pawn))))) AxisValue false))

(event Input|AxisEvents|InputAxisTurnn
  (params (AxisValue :type Float%20%28single-precision%29))
  ;[1 1 1] camera
  (Pawn|Input|AddControllerYawInput AxisValue))

(event Input|AxisEvents|InputAxisLookUpp
  (params (AxisValue :type Float%20%28single-precision%29))
  ;[1 1 1] camera
  (Pawn|Input|AddControllerPitchInput AxisValue))

(fn ConstructionScript)

(fn Infligdegat
  (params (pointdegat :type Float%20%28single-precision%29))
  (Variables|Default|Setvie (Math|Float|Clamp(Float) (- (Variables|Default|Getvie) pointdegat) 0.0 (Variables|Default|GetvieMax)))
  (if (not (> (Variables|Default|Getvie) 0.0))
    (CallFunction|Mort)))

(fn RendVie
  (params (pointdevie :type Float%20%28single-precision%29))
  (Variables|Default|Setvie (Math|Float|Clamp(Float) (+ (Variables|Default|Getvie) pointdevie) 0.0 (Variables|Default|GetvieMax))))

(fn Mort
  (Input|DisableInput (Game|GetPlayerController 0))
  (Components|Animation|PlayAnimation (Variables|Character|GetMesh) "/Game/Personnage/animation/death.death" false)
  (Audio|PlaySound2D "/Game/StarterContent/Audio/Explosion01.Explosion01" 1.0 1.0 0.0 0 0))

(fn RamasserItem
  (bind _camera (Variables|Default|GetCamera))
  (bind _camera_2 (Variables|Default|GetCamera))
  (bind (_outhit _returnvalue) (Collision|SphereTraceByChannel (+ (Transformation|GetWorldLocation _camera) (* (Math|Vector|GetForwardVector _camera) 330)) (+ (Transformation|GetWorldLocation _camera_2) (* (Math|Vector|GetForwardVector _camera_2) 550)) 25.0 "TraceTypeQuery1" false 0 "None"))
  (if _returnvalue
    (bind _asbp_main_item (Utilities|Casting|CastToBP_main_Item (.HitActor (Collision|BreakHitResult _outhit))))
    (CallFunction|AddItem _asbp_main_item)))

(fn AddItem
  (params (itemRef :type BP%20Main%20Item%20Object%20Reference))
  (bind _output_get (Variables|Default|Setitem%20Struct%20Ref (Variables|/Game/Items/BP_main_Item.BP_main_Item_C|Gets_item itemRef)))
  (if (Utilities|Struct|BreakS_items _output_get)
    (bind (_array_element _array_index) (Utilities|Array|ForEachLoopwithBreak (Variables|Default|Getinventaire) :!label _label)
      (:LoopBody
        (if (Utilities|Enum|Equal(Enum) (Utilities|Struct|BreakS_items _array_element) (Utilities|Struct|BreakS_items (Variables|Default|Getitem%20Struct%20Ref)))
          (LocalVariables|Setitem%20trouvé%20? true)
          (goto _label Break)))
      (:Completed
        (if (LocalVariables|Getitem%20trouvé%20?)
          (Utilities|Array|SetArrayElem (Variables|Default|Getinventaire) _array_index (Utilities|Struct|MakeS_items (.nom (Utilities|Struct|BreakS_items _array_element)) (.description (Utilities|Struct|BreakS_items _array_element)) (.image (Utilities|Struct|BreakS_items _array_element)) (.isStackable? (Utilities|Struct|BreakS_items _array_element)) (.type (Utilities|Struct|BreakS_items _array_element)) (.bonus (Utilities|Struct|BreakS_items _array_element)) (+ (.nombre (Utilities|Struct|BreakS_items _array_element)) 1)))
          (Actor|DestroyActor itemRef)
          (CallFunction|ChargerInventaire)
          (else
            (Utilities|Array|Add (Variables|Default|Getinventaire) (Variables|/Game/Items/BP_main_Item.BP_main_Item_C|Gets_item itemRef) :!label _label_2)
            (Actor|DestroyActor itemRef)
            (CallFunction|ChargerInventaire)))))
    (else
      (goto _label_2))))

(fn ChargerInventaire
  (Utilities|IsValid (Variables|Default|GetUI_BagRef)
    (:Is%20Valid
      (Widget|Panel|ClearChildren (Variables|/Game/HUD/UI_bag.UI_bag_C|GetVerticalBoxBag (Variables|Default|GetUI_BagRef)))
      (for _array_element (Variables|Default|Getinventaire)
        (bind _returnvalue (UserInterface|CreateWidget "/Game/HUD/UI_item.UI_item_C" 0 _array_element))
        (Class|VerticalBox|AddChildtoVerticalBox (Variables|/Game/HUD/UI_bag.UI_bag_C|GetVerticalBoxBag (Variables|Default|GetUI_BagRef)) _returnvalue)))))