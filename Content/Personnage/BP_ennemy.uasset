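; BP_ennemy is an enemy character Blueprint that takes damage and dies.
; The Infligdegat event subtracts incoming damage points from Vie, clamped between zero and VieMax.
; While health remains it plays a front hit-reaction montage on the mesh; otherwise it calls Mort and deactivates CharacterMovement.
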(event EventInfligdegat
  (params (pointdegat :type Float%20%28single-precision%29))
  (Variables|Default|Setvie (Math|Float|Clamp(Float) (- (Variables|Default|Getvie) pointdegat) 0.0 (Variables|Default|GetvieMax)))
  (if (> (Variables|Default|Getvie) 0.0)
    (Animation|Montage|PlayMontage (Variables|Character|GetMesh) "/Game/Personnage/animation/Standing_React_Large_From_Front_Montage.Standing_React_Large_From_Front_Montage")
    (else
      (CallFunction|Mort)
      (Components|Activation|Deactivate (Variables|Character|GetCharacterMovement)))))

(fn ConstructionScript
  (|CallParentFunction))