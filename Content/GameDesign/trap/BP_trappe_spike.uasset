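; BP_trappe_spike is a spike trap that kills the player's paladin on contact with its trigger box.
; Overlap by a BP_paladin plays timelines that move the pressure plate and spikes vertically, and immediately calls Mort on player 0's paladin.
; Ending the overlap reverses both timelines.
; The construction script builds the spikes as a 4x4 grid of evenly spaced instances.
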(event OnComponentBeginOverlap(Box)
  (params (OverlappedComponent :type Primitive%20Component%20Object%20Reference) (OtherActor :type Actor%20Object%20Reference) (OtherComp :type Primitive%20Component%20Object%20Reference) (OtherBodyIndex :type Integer) (bFromSweep :type Boolean) (SweepResult :type Hit%20Result%20Structure%20%28by%20ref%29))
  (Utilities|Casting|CastToBP_paladin OtherActor)
  (Utilities|FlowControl|Sequence
    (:then_0
      (bind _hauteur (Timeline|PlaqueDown PlayFromStart)
        (:Update
          (Transformation|SetRelativeLocation (Variables|Default|GetPlaque%20int) (Math|Vector|MakeVector 0.0 0.0 _hauteur) false false))))
    (:then_1
      (bind _newtrack_0 (Timeline|pick%20up PlayFromStart)
        (:Update
          (Transformation|SetRelativeLocation (Variables|Default|GetPics) (Math|Vector|MakeVector -1.1e+02 -106.0 _newtrack_0) false false))))
    (:then_2
      (bind _asbp_paladin (Utilities|Casting|CastToBP_paladin (Game|GetPlayerCharacter 0)))
      (Default|Mort _asbp_paladin))))

(event OnComponentEndOverlap(Box)
  (params (OverlappedComponent :type Primitive%20Component%20Object%20Reference) (OtherActor :type Actor%20Object%20Reference) (OtherComp :type Primitive%20Component%20Object%20Reference) (OtherBodyIndex :type Integer))
  (Utilities|Casting|CastToBP_paladin OtherActor)
  (Utilities|FlowControl|Sequence
    (:then_0
      (bind _hauteur (Timeline|PlaqueDown ReverseFromEnd)
        (:Update
          (Transformation|SetRelativeLocation (Variables|Default|GetPlaque%20int) (Math|Vector|MakeVector 0.0 0.0 _hauteur) false false))))
    (:then_1
      (bind _newtrack_0 (Timeline|pick%20up ReverseFromEnd)
        (:Update
          (Transformation|SetRelativeLocation (Variables|Default|GetPics) (Math|Vector|MakeVector -1.1e+02 -106.0 _newtrack_0) false false))))))

(fn ConstructionScript
  (for _index (range 0 3)
    (for _index_2 (range 0 3)
      (Components|InstancedStaticMesh|AddInstance (Variables|Default|GetPics) (Math|Transform|MakeTransform (* (Math|Vector|MakeVector (Math|Conversions|ToFloat(Integer) _index) (Math|Conversions|ToFloat(Integer) _index_2) 0.0) 180))))))