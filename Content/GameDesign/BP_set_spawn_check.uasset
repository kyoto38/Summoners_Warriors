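; Trigger-box Blueprint that kills the overlapping paladin and respawns the player at a fixed checkpoint location.
; On overlap it disables input, plays a death animation and explosion sound, then after a delay spawns a new BP_paladin at hard-coded coordinates and possesses it.
; CountCheckpoint is set without waiting for the delay, so the trigger fires only once, and the old pawn is left undestroyed.
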(event OnComponentBeginOverlap(Box)
  (params (OverlappedComponent :type Primitive%20Component%20Object%20Reference) (OtherActor :type Actor%20Object%20Reference) (OtherComp :type Primitive%20Component%20Object%20Reference) (OtherBodyIndex :type Integer) (bFromSweep :type Boolean) (SweepResult :type Hit%20Result%20Structure%20%28by%20ref%29))
  (if (not (Variables|Default|Getcount_checkpoint))
    (bind _asbp_paladin (Utilities|Casting|CastToBP_paladin OtherActor))
    (Utilities|FlowControl|Sequence
      (:then_0
        (Input|DisableInput _asbp_paladin (Game|GetPlayerController 0))
        (Components|Animation|PlayAnimation (Variables|/Script/Engine.Character|GetMesh _asbp_paladin) "/Game/Personnage/animation/death.death" false)
        (Audio|PlaySound2D "/Game/StarterContent/Audio/Explosion01.Explosion01" 1.0 1.0 0.0 0 0))
      (:then_1
        (Utilities|FlowControl|Delay 3.0)
        (bind _returnvalue (Game|SpawnActorfromClass "/Game/Personnage/BP_paladin.BP_paladin_C" (Math|Transform|MakeTransform "-13110.914062,35316.417969,860.268188" "0, 0, 0" "1,1,1") "Undefined" 0 0))
        (Pawn|Possess (Game|GetPlayerController 0) _returnvalue))
      (:then_2
        (Variables|Default|Setcount_checkpoint true)))))

(fn ConstructionScript)